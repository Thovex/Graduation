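; BP_WFC is a debug harness actor for 3D Wave Function Collapse generation, driven by keyboard keys.
; From BeginPlay, the self-repeating Blien event draws each cell's allowed-pattern count as world-space debug text, refreshing via a 0.2-second Delay.
; Keys initialize the wave, run a full solve from preset JSON, observe the minimum-entropy cell, solve then call JsonExport's ParseData, or create from saved JSON.
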(event Custom|Blien
  (bind _wave (Variables|Default|GetWave))
  (bind _array3d (Utilities|Struct|BreakWaveMatrix _wave))
  (bind _keys (Utilities|Map|Keys _array3d))
  (bind _values (Utilities|Map|Values _array3d))
  (for (_array_element _array_index) _keys
    (Variables|Default|SetCount 0)
    (bind _values_2 (Utilities|Map|Values (Utilities|Struct|BreakCoefficient (Utilities|Array|Get(acopy) _values _array_index))))
    (for _array_element_2 _values_2
      (if _array_element_2
        (Math|Integer|IncrementInt (Variables|Default|GetCount))))
    (Rendering|Debug|DrawDebugString (+ (Transformation|GetActorLocation) (* (Math|Conversions|ToVector(Float) _array_element) 1e+03)) (Utilities|String|ToString(Integer) (Variables|Default|GetCount)) 0 "(R=1.000000,G=0.000000,B=0.215879,A=1.000000)" 0.2)
    (Utilities|FlowControl|Delay 0.2)
    (CallFunction|Blien)))

(event EventBeginPlay
  (|CallParentFunction)
  (CallFunction|Blien))

(event EventTick
  (params (DeltaSeconds :type Float%20%28single-precision%29))
  (|CallParentFunction DeltaSeconds))

(event Input|KeyboardEvents|Up
  (params (Key :type Key%20Structure))
  (:Pressed
    (bind _returnvalue (Class|WFC|MinEntropyCoords))
    (Class|WFC|Observe _returnvalue -1)))

(event Input|KeyboardEvents|I
  (params (Key :type Key%20Structure))
  (:Pressed
    (Class|WFC|Initialize)))

(event Input|KeyboardEvents|J
  (params (Key :type Key%20Structure))
  (:Pressed
    (Class|WFC|StartWFC)
    (Class|JsonExporter|ParseData (Variables|Default|GetJsonExport) (Variables|Default|GetWave) (Variables|Default|GetModuleAssignee))))

(event Input|KeyboardEvents|P
  (params (Key :type Key%20Structure))
  (:Pressed
    (bind _returnvalue (Class|JsonExporter|RetrieveDataFileName (Variables|Default|GetJsonExport) "WFC_2x2x2_2019.05.19-17.18.31" true))
    (Class|WFC|CreatefromJson _returnvalue)))

(event Input|KeyboardEvents|SpaceBar
  (params (Key :type Key%20Structure))
  (:Pressed
    (Class|WFC|Initialize)
    (bind _returnvalue (Class|JsonExporter|RetrieveDataFileName (Variables|Default|GetJsonExport) "WFC_2x2x2_2019.05.19-17.21.17.json" true))
    (Class|WFC|FillInitialData _returnvalue)
    (Class|WFC|StartWFC)))

(fn ConstructionScript
  (|CallParentFunction))