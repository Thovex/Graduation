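; BP_M_TunnelTube is a tunnel tube module Blueprint that randomly removes its particle effect for variation.
; StartEvent makes two independent coin flips, each able to destroy the same ParticleSystem1 component if it is still valid.
; It runs in the construction script and again after a short delay following BeginPlay, both after the parent logic, so removal odds compound.
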(event EventBeginPlay
  (|CallParentFunction)
  (Utilities|FlowControl|Delay 2.0)
  (CallFunction|StartEvent))

(fn ConstructionScript
  (|CallParentFunction)
  (CallFunction|StartEvent))

(fn StartEvent
  (bind _particlesystem1 (Variables|Default|GetParticleSystem1))
  (bind _particlesystem1_2 (Variables|Default|GetParticleSystem1))
  (Utilities|FlowControl|Sequence
    (:then_0
      (if (Math|Random|RandomBool)
        (Utilities|IsValid _particlesystem1_2
          (:Is%20Valid
            (Components|DestroyComponent _particlesystem1_2)))))
    (:then_1
      (if (Math|Random|RandomBool)
        (Utilities|IsValid _particlesystem1
          (:Is%20Valid
            (Components|DestroyComponent _particlesystem1)))))))