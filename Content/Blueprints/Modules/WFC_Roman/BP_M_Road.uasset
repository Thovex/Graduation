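; Modular road piece in the Roman WFC set that picks its own mesh to match adjacent road pieces.
; StartEvent line-traces four ways for non-excluded roads, matches connected sides against RoadSideSelector to set mesh and type, then tallies neighbour types.
; PostStartEvent turns qualifying junctions into four-way centre meshes, occasionally with a statue, excludes them from tracing and re-runs both passes on neighbours, letting changes cascade.
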(event EventConstruct
  (|CallParentFunction)
  (CallFunction|StartEvent))

(fn ConstructionScript
  (|CallParentFunction)
  (CallFunction|StartEvent))

(fn TraceAllSides
  (bind _trace (Variables|Default|GetTrace))
  (bind _returnvalue (Transformation|GetWorldLocation _trace))
  (Utilities|Map|Clear (Variables|Default|GetTraceNeighbours))
  (for _array_element (Variables|Default|GetTraceSides)
    (bind _outhit (Collision|LineTraceByChannel _returnvalue (+ _returnvalue (* (.Vector (Utilities|Struct|BreakFRoadSideData _array_element)) 1.5e+03)) "TraceTypeQuery3" false 0 "ForDuration" true "(R=0.000000,G=0.267617,B=1.000000,A=1.000000)"))
    (if (Utilities|ClassIsChildOf (Utilities|GetClass (.HitActor (Collision|BreakHitResult _outhit))) "BP_M_Road_C")
      (bind _asbp_m_road (Utilities|Casting|CastToBP_M_Road (.HitActor (Collision|BreakHitResult _outhit))))
      (if (not (Variables|BP_M_Road_C|GetExcluded _asbp_m_road))
        (Utilities|Map|Add (Variables|Default|GetTraceHits) (.Side (Utilities|Struct|BreakFRoadSideData _array_element)) true)
        (Utilities|Map|Add (Variables|Default|GetTraceNeighbours) (.Side (Utilities|Struct|BreakFRoadSideData _array_element)) _asbp_m_road)))))

(fn GetTraceSides
  (bind _trace (Variables|Default|GetTrace))
  (bind _returnvalue (Math|Vector|GetRightVector _trace))
  (bind _returnvalue_2 (Math|Vector|GetForwardVector _trace))
  (Utilities|Array|Clear (Variables|Default|GetTraceSides))
  (for _index (range 0 3)
    (Utilities|Array|Add (Variables|Default|GetTraceSides) (Utilities|Struct|MakeFRoadSideData (Utilities|Enum|ByteToEnumERoadSide (Math|Conversions|ToByte(Integer) _index)) (Utilities|Select :Index _index :Option%200 _returnvalue_2 :Option%201 _returnvalue :Option%202 (Math|Vector|NegateVector _returnvalue_2) :Option%203 (Math|Vector|NegateVector _returnvalue)))))
  (for _index_2 (range 0 3)
    (Utilities|Map|Add (Variables|Default|GetTraceHits) (Utilities|Enum|ByteToEnumERoadSide (Math|Conversions|ToByte(Integer) _index_2)) false)))

(fn TransformMesh
  (bind _tracehits (Variables|Default|GetTraceHits))
  (bind _values (Utilities|Map|Values _tracehits))
  (bind _keys (Utilities|Map|Keys _tracehits))
  (for (_array_element _array_index) _keys
    (if (Utilities|Array|Get(acopy) _values _array_index)
      (Utilities|Array|Add (LocalVariables|GetSelected) _array_element)))
  (bind _mesh (CallFunction|GetEqual (LocalVariables|GetSelected)))
  (Components|StaticMesh|SetStaticMesh (Variables|Default|GetRoad) _mesh))

(fn GetEqual
  (params (Selected :type Array%20of%20ERoadSide%20Enums :default "NewEnumerator0"))
  (for _array_element (Variables|Default|GetRoadSideSelector)
    (if (Class|UtilityLibrary|EqualByteArray Selected (.Sides (Utilities|Struct|BreakFRoadSideSelector _array_element)))
      (Variables|Default|SetType (.Type (Utilities|Struct|BreakFRoadSideSelector _array_element)))
      (return (.Mesh (Utilities|Struct|BreakFRoadSideSelector _array_element)))))
  (return "/Game/Meshes/World/Road/SM_Road_ForwardBack.SM_Road_ForwardBack"))

(fn StartEvent
  (CallFunction|GetTraceSides)
  (CallFunction|TraceAllSides)
  (CallFunction|TransformMesh)
  (CallFunction|GetNeighbourCounts))

(fn PostStartEvent
  (bind _typeneighbourcount (Variables|Default|GetTypeNeighbourCount))
  (CallFunction|GetNeighbourCounts)
  (Utilities|FlowControl|Sequence
    (:then_1
      (if (and (Utilities|Enum|Equal(Enum) (Variables|Default|GetType) "NewEnumerator3") (or (> (.Value (Utilities|Map|Find _typeneighbourcount "NewEnumerator3")) 1) (> (.Value (Utilities|Map|Find _typeneighbourcount "NewEnumerator2")) 2)))
        (CallFunction|CreateStatue)))))

(fn CreateStatue
  (bind _road (Variables|Default|GetRoad))
  (if (Math|Random|RandomBoolwithWeight 0.2)
    (Components|StaticMesh|SetStaticMesh _road "/Game/Meshes/World/Road/SM_Road_FBRL_StatueCenter.SM_Road_FBRL_StatueCenter")
    (else
      (Components|StaticMesh|SetStaticMesh _road "/Game/Meshes/World/Road/SM_Road_FBRL_NoStatueCenter.SM_Road_FBRL_NoStatueCenter")))
  (Variables|Default|SetExcluded true)
  (bind _values (Utilities|Map|Values (Variables|Default|GetTraceNeighbours)))
  (for _array_element _values
    (CallFunction|StartEvent _array_element))
  (for _array_element_2 _values
    (CallFunction|PostStartEvent _array_element_2)))

(fn GetNeighbourCounts
  (bind _typeneighbourcount (Variables|Default|GetTypeNeighbourCount))
  (Utilities|Map|Clear (Variables|Default|GetTypeNeighbourCount))
  (bind _values (Utilities|Map|Values (Variables|Default|GetTraceNeighbours)))
  (for _array_element _values
    (Utilities|Map|Add _typeneighbourcount (Variables|BP_M_Road_C|GetType _array_element) (+ (.Value (Utilities|Map|Find _typeneighbourcount (Variables|BP_M_Road_C|GetType _array_element))) 1))))