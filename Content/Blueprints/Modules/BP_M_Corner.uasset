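; BP_M_Corner is a corner module that labels itself with random letter-number text and adapts when stacked above another corner.
; StartEvent runs on construction and one second after BeginPlay, tracing down from Arrow for another BP_M_Corner.
; If one is found, it swaps to the upper mesh and removes text and lights.
; It then traces from Arrow's children, spawning cables to any Module-derived actors hit, sized by hit distance plus slack.
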(event EventBeginPlay
  (|CallParentFunction)
  (Utilities|FlowControl|Delay 1.0)
  (CallFunction|StartEvent))

(fn ConstructionScript
  (|CallParentFunction)
  (CallFunction|StartEvent))

(fn StartEvent
  (Utilities|FlowControl|Sequence
    (:then_0
      (CallFunction|SetCornerText))
    (:then_1
      (bind _returnvalue (CallFunction|TraceDowntoCheckforCorner))
      (if _returnvalue
        (CallFunction|AdjustMeshandRemoveComponents)
        (CallFunction|AssignCableComponents)
        (CallFunction|CableTraceandCreate)))))

(fn SetCornerText
  (bind _textrender (Variables|Default|GetTextRender))
  (Utilities|IsValid _textrender
    (:Is%20Valid
      (Rendering|Components|TextRender|SetText _textrender (Utilities|Text|FormatText "{Row} | {Number}" (Utilities|Select :Index (Math|Random|RandomIntegerinRange 0 3) :Option%200 (Utilities|Text|MakeLiteralText "A") :Option%201 (Utilities|Text|MakeLiteralText "B") :Option%202 (Utilities|Text|MakeLiteralText "C") :Option%203 (Utilities|Text|MakeLiteralText "D")) (Math|Random|RandomIntegerinRange 0 999))))))

(fn TraceDowntoCheckforCorner
  (bind _arrow (Variables|Default|GetArrow))
  (bind _returnvalue (Transformation|GetWorldLocation _arrow))
  (bind _outhit (Collision|LineTraceByChannel _returnvalue (+ _returnvalue (* (Math|Vector|VectorDown) 1e+04)) "TraceTypeQuery1" false 0 "None" true "(R=1.000000,G=0.000000,B=0.000000,A=1.000000)" "(R=0.000000,G=1.000000,B=0.000000,A=1.000000)" 25.0))
  (return (== (Utilities|GetClass (.HitActor (Collision|BreakHitResult _outhit))) "BP_M_Corner_C")))

(fn AdjustMeshandRemoveComponents
  (bind _textrender (Variables|Default|GetTextRender))
  (bind _rectlight (Variables|Default|GetRectLight))
  (bind _rectlight1 (Variables|Default|GetRectLight1))
  (Components|StaticMesh|SetStaticMesh (Variables|Default|GetSM%20Corner) "/Game/Meshes/WFC/V02/SM_Corner_Up_v02.SM_Corner_Up_v02")
  (Utilities|FlowControl|Sequence
    (:then_0
      (Utilities|IsValid _textrender
        (:Is%20Valid
          (Components|DestroyComponent _textrender))))
    (:then_1
      (Utilities|IsValid _rectlight
        (:Is%20Valid
          (Components|DestroyComponent _rectlight))))
    (:then_2
      (Utilities|IsValid _rectlight1
        (:Is%20Valid
          (Components|DestroyComponent _rectlight1))))))

(fn AssignCableComponents
  (Variables|Default|SetCableLocations (Components|GetChildrenComponents (Variables|Default|GetArrow) false)))

(fn CableTraceandCreate
  (for _array_element (Variables|Default|GetCableLocations)
    (bind (_outhit _returnvalue) (Collision|LineTraceByChannel (Transformation|GetWorldLocation _array_element) (+ (Transformation|GetWorldLocation _array_element) (* (Math|Vector|GetForwardVector _array_element) 2e+03)) "TraceTypeQuery1" false 0 "None" true "(R=1.000000,G=0.000000,B=0.000000,A=1.000000)" "(R=0.000000,G=1.000000,B=0.000000,A=1.000000)" 15.0))
    (if _returnvalue
      (if (Utilities|ClassIsChildOf (Utilities|GetClass (.HitActor (Collision|BreakHitResult _outhit))) "/Script/AndromedaResonance.Module")
        (bind _returnvalue_2 (AddComponent|AddCableComponent false))
        (Transformation|AttachComponentToComponent _returnvalue_2 _array_element "None" "SnapToTarget" "SnapToTarget" "SnapToTarget" true)
        (bind _returnvalue_3 (AddComponent|AddSceneComponent (.HitActor (Collision|BreakHitResult _outhit)) false))
        (Transformation|SetWorldLocation _returnvalue_3 (+ (.ImpactPoint (Collision|BreakHitResult _outhit)) (* (Math|Vector|GetForwardVector _array_element) 1.5e+02)) false false)
        (Class|CableComponent|SetAttachEndtoComponent _returnvalue_2 _returnvalue_3 "None")
        (Variables|/Script/CableComponent.CableComponent|SetCableLength _returnvalue_2 (+ (.Distance (Collision|BreakHitResult _outhit)) 2e+02))))))