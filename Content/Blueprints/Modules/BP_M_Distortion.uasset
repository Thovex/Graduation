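; Distortion zone module that disrupts the BP_HeliSphere drone inside its box and advances encryption progress if it carries collected data, resetting that progress on exit.
; Overlap toggles HUD distortion, Chameleon camera shake and glitch, and a looping timer for random force, spin and brief drone shutdowns.
; Tick ramps intensity with time spent inside, feeding the HUD and the XIntensity scaling of those disturbances.
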(event OnComponentBeginOverlap(Box_0)
  (params (OverlappedComponent :type Primitive%20Component%20Object%20Reference) (OtherActor :type Actor%20Object%20Reference) (OtherComp :type Primitive%20Component%20Object%20Reference) (OtherBodyIndex :type Integer) (bFromSweep :type Boolean) (SweepResult :type Hit%20Result%20Structure%20%28by%20ref%29))
  (bind _chameleon (Variables|Default|GetChameleon))
  (bind _asbp_heli_sphere (Utilities|Casting|CastToBP_HeliSphere OtherActor))
  (Utilities|FlowControl|Sequence
    (:then_0
      (Variables|Default|SetDroneInside true)
      (bind _returnvalue (Utilities|Time|SetTimerbyEvent (EventDispatchers|CreateEvent :!event Custom|ApplyForce) 0.15 true))
      (Variables|Default|SetTimerHandle _returnvalue))
    (:then_1
      (bind _output_get (Variables|Default|SetDrone _asbp_heli_sphere))
      (Utilities|IsValid (Variables|/Game/Blueprints/Gameplay/BP_HeliSphere.BP_HeliSphere_C|GetHUD _output_get)
        (:Is%20Valid
          (Default|Distort (Variables|/Game/Blueprints/Gameplay/BP_HeliSphere.BP_HeliSphere_C|GetHUD _output_get) true))))
    (:then_2
      (Utilities|IsValid _chameleon
        (:Is%20Valid
          (Variables|/Game/Chameleon/Chameleon.Chameleon_C|SetCamera%20Shake _chameleon true)
          (Variables|/Game/Chameleon/Chameleon.Chameleon_C|SetGlitch _chameleon true))))))

(event OnComponentEndOverlap(Box_0)
  (params (OverlappedComponent :type Primitive%20Component%20Object%20Reference) (OtherActor :type Actor%20Object%20Reference) (OtherComp :type Primitive%20Component%20Object%20Reference) (OtherBodyIndex :type Integer))
  (bind _chameleon (Variables|Default|GetChameleon))
  (bind _asbp_heli_sphere (Utilities|Casting|CastToBP_HeliSphere OtherActor))
  (Utilities|FlowControl|Sequence
    (:then_0
      (Variables|Default|SetDroneInside false)
      (Utilities|Time|ClearandInvalidateTimerbyHandle (Variables|Default|GetTimerHandle)))
    (:then_1
      (Utilities|IsValid (Variables|Default|GetChameleon)
        (:Is%20Valid
          (Variables|/Game/Chameleon/Chameleon.Chameleon_C|SetCamera%20Shake _chameleon false)
          (Variables|/Game/Chameleon/Chameleon.Chameleon_C|SetGlitch _chameleon false))))
    (:then_2
      (Utilities|IsValid (Variables|/Game/Blueprints/Gameplay/BP_HeliSphere.BP_HeliSphere_C|GetHUD _asbp_heli_sphere)
        (:Is%20Valid
          (Default|Distort (Variables|/Game/Blueprints/Gameplay/BP_HeliSphere.BP_HeliSphere_C|GetHUD _asbp_heli_sphere) false))))
    (:then_3
      (Variables|/Game/Blueprints/Gameplay/BP_HeliSphere.BP_HeliSphere_C|SetEncryptedDataProgress _asbp_heli_sphere 0.0))))

(event Custom|ApplyForce
  (bind _drone (Variables|Default|GetDrone))
  (bind _drone_2 (Variables|Default|GetDrone))
  (bind _helisphere (Variables|/Game/Blueprints/Gameplay/BP_HeliSphere.BP_HeliSphere_C|GetHeliSphere _drone))
  (if (Variables|Default|GetDroneInside)
    (Physics|AddRadialForce _helisphere (Math|Random|RandomPointinBoundingBox (Transformation|GetWorldLocation (Variables|Default|GetBox_0)) "1000.000000,1000.000000,1000.000000") (Variables|Default|GetRadius) (Utilities|XIntensity (Variables|Default|GetForce)) "RIF_Constant" true)
    (Class|PrimitiveComponent|AddAngularImpulseinDegrees _helisphere (* (Math|Random|RandomUnitVector) (Utilities|XIntensity (Math|Random|RandomFloatinRange 1e+02 2e+02))) "None" true)
    (if (Math|Random|RandomBoolwithWeight 0.02)
      (Default|SetActive _drone_2 false)
      (Utilities|FlowControl|Delay (Utilities|XIntensity (Math|Random|RandomFloatinRange 0.2 0.7)))
      (Default|SetActive _drone_2 true))))

(event EventTick
  (params (DeltaSeconds :type Float%20%28single-precision%29))
  (bind _drone (Variables|Default|GetDrone))
  (if (Variables|Default|GetDroneInside)
    (bind _output_get (Variables|Default|SetSecondsInside (+ (Variables|Default|GetSecondsInside) DeltaSeconds)))
    (bind _output_get_2 (Variables|Default|SetIntensity (Class|UtilityLibrary|SetScalePure (Math|Float|Clamp(Float) _output_get 0.0 1e+01) 0.0 1e+01 (Variables|Default|GetMinIntensity) (Variables|Default|GetMaxIntensity))))
    (Variables|/Game/Blueprints/Widgets/Game/WBP_Drone_UI.WBP_Drone_UI_C|SetDistortionIntensity (Variables|/Game/Blueprints/Gameplay/BP_HeliSphere.BP_HeliSphere_C|GetHUD _drone) _output_get_2)
    (if (Variables|/Game/Blueprints/Gameplay/BP_HeliSphere.BP_HeliSphere_C|GetbCollectedData _drone)
      (Default|AddEncryptionProgress _drone))
    (else
      (Variables|Default|SetSecondsInside 0.0))))

(event EventBeginPlay
  (|CallParentFunction)
  (bind _outactors (Actor|GetAllActorsOfClass "/Game/Chameleon/Chameleon.Chameleon_C"))
  (Variables|Default|SetChameleon (Utilities|Array|Get(acopy) _outactors)))

(fn ConstructionScript
  (|CallParentFunction))