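; BP_M_Radar is a radar module that feeds data to BP_HeliSphere from a finite, randomized reserve.
; A RotatingMovement component targets the mesh, which starts at a random yaw.
; Each Tick box-traces forward from Trace; hitting a HeliSphere with incomplete progress adds progress and drains DataLeft.
; DataLeft also sizes the box, so coverage shrinks as it depletes, and the Inside flag toggles debug drawing.
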(event EventBeginPlay
  (|CallParentFunction)
  (Components|Movement|SetUpdatedComponent (Variables|Default|GetRotatingMovement) (Variables|Default|GetStaticMesh1))
  (Transformation|SetWorldRotation (Variables|Default|GetStaticMesh1) (Math|Rotator|MakeRotator 0.0 0.0 (Math|Random|RandomFloatinRange 0.0 3.6e+02)) false false)
  (Variables|Default|SetDataLeft (Math|Random|RandomFloatinRange 45.0 115.0)))

(event EventTick
  (params (DeltaSeconds :type Float%20%28single-precision%29))
  (bind _trace (Variables|Default|GetTrace))
  (bind _returnvalue (Transformation|GetWorldLocation _trace))
  (bind (_outhit _returnvalue_2) (Collision|BoxTraceByChannel _returnvalue (+ _returnvalue (* (Math|Vector|GetForwardVector _trace) 1e+04)) (Math|Vector|MakeVector (Variables|Default|GetDataLeft) (Variables|Default|GetDataLeft) (Variables|Default|GetDataLeft)) (Transformation|GetWorldRotation (Variables|Default|GetTrace)) "TraceTypeQuery1" false 0 (select (Variables|Default|GetInside) "ForOneFrame" "None")))
  (if _returnvalue_2
    (if (== (Utilities|GetClass (.HitActor (Collision|BreakHitResult _outhit))) "/Game/Blueprints/Gameplay/BP_HeliSphere.BP_HeliSphere_C")
      (bind _asbp_heli_sphere (Utilities|Casting|CastToBP_HeliSphere (.HitActor (Collision|BreakHitResult _outhit))))
      (if (< (Variables|/Game/Blueprints/Gameplay/BP_HeliSphere.BP_HeliSphere_C|GetCollectedDataProgress _asbp_heli_sphere) 1e+02)
        (if (> (Variables|Default|GetDataLeft) 0.0)
          (Default|AddDataProgress _asbp_heli_sphere)
          (Variables|Default|SetDataLeft (- (Variables|Default|GetDataLeft) 0.1))
          (Variables|Default|SetInside true))))
    (else
      (Variables|Default|SetInside false))))

(fn ConstructionScript
  (|CallParentFunction))