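; World manager that moves static meshes of allowed module actors from BP_WFC generation into instancing via AppendMesh, hiding the originals.
; On BeginPlay it registers with the WFC actor, then waits briefly after post-production finishes and scans the spawned child actors.
; It accepts only exact StaticMeshComponents there, substituting a fixed scale for zero-scale transforms.
; AppendHISMArrayActors does the same for a supplied actor array, skipping only spline meshes, without the scale fix.
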(event Custom|AcquireHISMs
  (Utilities|FlowControl|Delay 1.0)
  (bind _values (Utilities|Map|Values (Variables|/Script/AndromedaResonance.WFC|GetSpawnedComponents (Variables|Default|GetBP_WFC))))
  (for _array_element _values
    (if (Class|HISMManager|IsValid _array_element)
      (if (Utilities|Array|ContainsItem (Variables|Default|GetModules) (Utilities|GetClass (Variables|/Script/Engine.ChildActorComponent|GetChildActor _array_element)))
        (for _array_element_2 (Actor|GetComponentsByClass (Variables|/Script/Engine.ChildActorComponent|GetChildActor _array_element) "/Script/Engine.StaticMeshComponent")
          (if (not (!= (Utilities|GetClass _array_element_2) "/Script/Engine.StaticMeshComponent"))
            (Class|HISMManager|AppendMesh (select (Math|Vector|Equal(Vector) (.Scale (Math|Transform|BreakTransform (Transformation|GetWorldTransform _array_element_2))) "0, 0, 0" 0.0001) (Math|Transform|MakeTransform (.Location (Math|Transform|BreakTransform (Transformation|GetWorldTransform _array_element_2))) (.Rotation (Math|Transform|BreakTransform (Transformation|GetWorldTransform _array_element_2))) "10.000000,10.000000,10.000000") (Transformation|GetWorldTransform _array_element_2)) (Variables|/Script/Engine.StaticMeshComponent|GetStaticMesh _array_element_2) (Rendering|Material|GetMaterials _array_element_2))
            (Rendering|SetVisibility _array_element_2 false false)))))))

(event Custom|AppendHISMArrayActors
  (params (ActorAray :type Array%20of%20Actor%20Object%20References))
  (for _array_element ActorAray
    (if (Class|HISMManager|IsValid _array_element)
      (if (Utilities|Array|ContainsItem (Variables|Default|GetModules) (Utilities|GetClass _array_element))
        (for _array_element_2 (Actor|GetComponentsByClass _array_element "/Script/Engine.StaticMeshComponent")
          (if (not (== (Utilities|GetClass _array_element_2) "/Script/Engine.SplineMeshComponent"))
            (Class|HISMManager|AppendMesh (Transformation|GetWorldTransform _array_element_2) (Variables|/Script/Engine.StaticMeshComponent|GetStaticMesh _array_element_2) (Rendering|Material|GetMaterials _array_element_2))
            (Rendering|SetVisibility _array_element_2 false false)))))))

(event EventBeginPlay
  (bind _wfc (Variables|Default|GetWFC))
  (|CallParentFunction)
  (Utilities|IsValid _wfc
    (:Is%20Valid
      (bind _asbp_wfc (Utilities|Casting|CastToBP_WFC _wfc))
      (bind _output_get (Variables|Default|SetBP_WFC _asbp_wfc))
      (Variables|/Game/Blueprints/WFC/BP_WFC.BP_WFC_C|SetHISMManager _output_get self)
      (EventDispatchers|BindEventtoFinishedPostProduction _output_get (delegate Custom|AcquireHISMs)))))

(fn ConstructionScript)