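; BP_DataGrid is a placeable grid actor whose construction script shows its own display name on a text component.
; When its Errors list is empty, a DoOnce gate destroys and clears the DisplayModules components, then calls DisplayRotatedPatterns to rebuild them.
; The pattern display is built at construction time, so it previews in the editor.
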(fn ConstructionScript
  (bind _displaymodules (Variables|Default|GetDisplayModules))
  (|CallParentFunction)
  (Rendering|Components|TextRender|SetText (Variables|Default|GetNameTR) (Utilities|Text|ToText(String) (Utilities|GetDisplayName self)))
  (if (== (Utilities|Map|Length (Variables|Default|GetErrors)) 0)
    (Utilities|FlowControl|DoOnce false
      (:Completed
        (for _array_element _displaymodules
          (Components|DestroyComponent _array_element))
        (Utilities|Array|Clear _displaymodules)
        (Class|DataGrid|DisplayRotatedPatterns)))))