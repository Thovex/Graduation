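; BP_PatternDisplay is a debug actor that lays out the patterns held by its ModuleAssignee for viewing in the world.
; Pressing End destroys the components from the previous display, then passes each pattern in the ModuleAssignee's map to CreatePatternData.
; Each pattern is offset at even intervals along the actor's right vector, and the returned components are stored for the next rebuild.
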(event Input|KeyboardEvents|End
  (params (Key :type Key%20Structure))
  (:Pressed
    (for _array_element (Variables|Default|GetPatterns)
      (Components|DestroyComponent _array_element))
    (Utilities|Array|Clear (Variables|Default|GetPatterns))
    (bind _values (Utilities|Map|Values (Variables|/Script/AndromedaResonance.ModuleAssignee|GetPatterns (Variables|Default|GetModuleAssignee))))
    (for (_array_element_2 _array_index) _values
      (bind _returnvalue (Class|WaveFunctionLibrary|CreatePatternData self (Variables|Default|GetModuleAssignee) _array_element_2 (+ (Transformation|GetActorLocation) (* (* (Transformation|GetActorRightVector) 3e+03) _array_index))))
      (for _array_element_3 _returnvalue
        (Utilities|Array|Add (Variables|Default|GetPatterns) _array_element_3)))))

(fn ConstructionScript)