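; BP_CameraRotation is a camera actor that takes over the first player's view and loops along a spline while facing a LookAt target.
; On BeginPlay it writes post-process depth-of-field settings (BokehDOF method) and blends the view to itself.
; A self-restarting timeline maps its alpha to spline distance, moving the camera and aiming it with FindLookAtRotation each update.
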(event Custom|StartTimeline
  (bind _spline (Variables|Default|GetSpline))
  (bind _camera (Variables|Default|GetCamera))
  (bind _alpha (Timeline|Timeline_0 PlayFromStart)
    (:Update
      (Transformation|SetWorldLocationAndRotation _camera (Spline|GetLocationatDistanceAlongSpline _spline (Class|UtilityLibrary|SetScalePure _alpha 0.0 1.0 0.0 (Spline|GetSplineLength _spline)) "World") (Math|Rotator|FindLookatRotation (Transformation|GetWorldLocation _camera) (Transformation|GetWorldLocation (Variables|Default|GetLookAt))) false false))
    (:Finished
      (CallFunction|StartTimeline))))

(event EventBeginPlay
  (Utilities|Struct|SetmembersinPostProcessSettings (Variables|/Game/Chameleon/Chameleon.Chameleon_C|GetNative%20Post%20Process (Variables|Default|GetChame)) "DOFM_BokehDOF")
  (Game|Player|SetViewTargetwithBlend (Game|GetPlayerController 0) self 0.1 "VTBlend_Linear" 0.0 false)
  (CallFunction|StartTimeline))

(fn ConstructionScript)