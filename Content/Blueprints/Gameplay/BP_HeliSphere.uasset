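; Player-controlled hover drone that moves as a physics sphere, with data collection and encryption progress and an in-game widget for distortion zones.
; Tick applies camera-relative forces, trace-based hover with adjustable height and tilt stabilization.
; Random line-trace scans draw beams and repel the drone from close surfaces.
; Stunt impulses and fast collisions, which briefly disable the drone, change the tint of lights and trails; stunts also raise loop pitch.
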(event OnComponentBeginOverlap(Box)
  (params (OverlappedComponent :type Primitive%20Component%20Object%20Reference) (OtherActor :type Actor%20Object%20Reference) (OtherComp :type Primitive%20Component%20Object%20Reference) (OtherBodyIndex :type Integer) (bFromSweep :type Boolean) (SweepResult :type Hit%20Result%20Structure%20%28by%20ref%29))
  (bind _returnvalue (Utilities|GetClass OtherActor))
  (bind _returnvalue_2 (Transformation|GetVelocity))
  (bind (_x _y _z) (Math|Vector|BreakVector _returnvalue_2))
  (if (and (!= _returnvalue "/Game/Blueprints/Modules/BP_M_Distortion.BP_M_Distortion_C") (!= _returnvalue "/Game/Blueprints/Gameplay/BP_Booster.BP_Booster_C"))
    (if (Math|Boolean|ORBoolean (> _x 5e+02) (> _y 5e+02) (> _z 5e+02))
      (Interactivity|SetActive false)
      (Math|Integer|IncrementInt (Variables|Stats|GetHitCount)
        (:%20%20
          (Utilities|FlowControl|Delay 3.0)
          (Interactivity|SetActive true))))
    (elif (Variables|Default|GetbCollectedData)
      (bind _returnvalue_3 (UserInterface|CreateWidget "/Game/Blueprints/Widgets/Game/WBP_Drone_InGame.WBP_Drone_InGame_C" 0 self))
      (UserInterface|Viewport|AddtoViewport _returnvalue_3 0)
      (Variables|Default|SetDroneGame _returnvalue_3)
      (Variables|Default|SetbInDistortion true))))

(event OnComponentEndOverlap(Box)
  (params (OverlappedComponent :type Primitive%20Component%20Object%20Reference) (OtherActor :type Actor%20Object%20Reference) (OtherComp :type Primitive%20Component%20Object%20Reference) (OtherBodyIndex :type Integer))
  (bind _returnvalue (Utilities|GetClass OtherActor))
  (bind _dronegame (Variables|Default|GetDroneGame))
  (if (not (and (!= _returnvalue "/Game/Blueprints/Modules/BP_M_Distortion.BP_M_Distortion_C") (!= _returnvalue "/Game/Blueprints/Gameplay/BP_Booster.BP_Booster_C")))
    (Variables|Default|SetbInDistortion false)
    (Utilities|IsValid _dronegame
      (:Is%20Valid
        (Default|Destroy _dronegame)))))

(event Custom|ScanRecursive
  (if (Variables|Physics|GetActive)
    (Physics|ScanSurroundings)))

(event EventBeginPlay
  (bind _dataabsorber (Variables|Default|GetDataAbsorber))
  (bind _scene4 (Variables|Default|GetScene4))
  (bind _scene2 (Variables|Default|GetScene2))
  (bind _scene3 (Variables|Default|GetScene3))
  (bind _scene1 (Variables|Default|GetScene1))
  (bind _array (Utilities|Array|MakeArray _scene1 _scene2 _scene3 _scene4))
  (bind _returnvalue (UserInterface|CreateWidget "/Game/Blueprints/Widgets/Game/WBP_Drone_UI.WBP_Drone_UI_C"))
  (UserInterface|Viewport|AddtoViewport _returnvalue 0)
  (Variables|Default|SetHUD _returnvalue)
  (Variables|Physics|SetLastLocation (Transformation|GetWorldLocation (Variables|Components|GetHeliSphere)))
  (Variables|/Script/AndromedaResonance.MultiRotatingMovementComponent|SetUpdatedComponents (Variables|Default|GetMultiRotatingMovement) _array)
  (Components|Movement|SetUpdatedComponent (Variables|Default|GetRotatingMovement) (Variables|Default|GetScene))
  (Utilities|Time|SetTimerbyEvent (EventDispatchers|CreateEvent :!event Custom|ScanRecursive) 0.25 true)
  (Effects|SpawnEmitterAttached "/Game/StarterContent/Particles/P_Ambient_Dust.P_Ambient_Dust" (Variables|Components|GetHeliSphere) "None" "0, 0, 0" "0, 0, 0" "2.000000,2.000000,2.000000")
  (for _array_element _array
    (bind _returnvalue_2 (Effects|SpawnEmitterAttached "/Game/Blueprints/Gameplay/VFX/PS_Trail.PS_Trail" _array_element "None" "0, 0, 0" "0, 0, 0" "2.000000,2.000000,2.000000"))
    (Utilities|Array|Add (Variables|Trail|GetTrails) _returnvalue_2)
    (bind _returnvalue_3 (Rendering|Material|CreateDynamicMaterialInstance (Rendering|Material|GetMaterial _returnvalue_2 0) "None" :!class /Script/Engine.KismetMaterialLibrary))
    (Utilities|Map|Add (Variables|Trail|GetTrailMaterials) _returnvalue_2 _returnvalue_3)
    (Rendering|Material|SetMaterial _returnvalue_2 0 _returnvalue_3))
  (bind _returnvalue_4 (Rendering|Material|CreateDynamicMaterialInstance (Rendering|Material|GetMaterial _dataabsorber 0) "None" :!class /Script/Engine.KismetMaterialLibrary))
  (Rendering|Material|SetMaterial _dataabsorber 0 _returnvalue_4)
  (Variables|Default|SetDataAbsorbMaterial _returnvalue_4))

(event EventTick
  (params (DeltaSeconds :type Float%20%28single-precision%29))
  (Interactivity|UpdateColor)
  (CallFunction|SoundInterp DeltaSeconds)
  (Interactivity|ColorImplementation)
  (if (Variables|Physics|GetActive)
    (Input|InputMove)
    (Input|InputUpDown)
    (Physics|Stabilize DeltaSeconds)
    (Physics|HoverUpdate)
    (Physics|AppendDistance)
    (CallFunction|KeepWingsZeroRotation)))

(event Input|AxisEvents|InputAxisLookUp
  (params (AxisValue :type Float%20%28single-precision%29))
  (Pawn|Input|AddControllerPitchInput AxisValue))

(event Input|AxisEvents|InputAxisTurn
  (params (AxisValue :type Float%20%28single-precision%29))
  (Pawn|Input|AddControllerYawInput AxisValue))

(event Input|KeyboardEvents|W
  (params (Key :type Key%20Structure))
  (:Pressed
    (Variables|Input|SetbW true))
  (:Released
    (Variables|Input|SetbW false)))

(event Input|KeyboardEvents|Q
  (params (Key :type Key%20Structure))
  (bind _returnvalue (Math|Random|RandomFloatinRange 2.5e+02 7.5e+02))
  (bind (_forward _right) (Utilities|ControllerForwardRightV))
  (bind _helisphere (Variables|Components|GetHeliSphere))
  (:Pressed
    (CallFunction|SetStunt true)
    (Physics|AddImpulse _helisphere (* _forward _returnvalue) "None" true)
    (Class|PrimitiveComponent|AddAngularImpulseinDegrees _helisphere (* _right _returnvalue) "None" true)
    (Utilities|FlowControl|Delay 1.0)
    (CallFunction|SetStunt false)))

(event Input|KeyboardEvents|S
  (params (Key :type Key%20Structure))
  (:Pressed
    (Variables|Input|SetbS true))
  (:Released
    (Variables|Input|SetbS false)))

(event Input|KeyboardEvents|A
  (params (Key :type Key%20Structure))
  (:Pressed
    (Variables|Input|SetbA true))
  (:Released
    (Variables|Input|SetbA false)))

(event Input|KeyboardEvents|D
  (params (Key :type Key%20Structure))
  (:Pressed
    (Variables|Input|SetbD true))
  (:Released
    (Variables|Input|SetbD false)))

(event Input|KeyboardEvents|SpaceBar
  (params (Key :type Key%20Structure))
  (:Pressed
    (Variables|Input|SetbSpace true))
  (:Released
    (Variables|Input|SetbSpace false)))

(event Input|KeyboardEvents|LeftCtrl
  (params (Key :type Key%20Structure))
  (:Pressed
    (Variables|Input|SetbCtrl true))
  (:Released
    (Variables|Input|SetbCtrl false)))

(event Input|KeyboardEvents|E
  (params (Key :type Key%20Structure))
  (bind _helisphere (Variables|Components|GetHeliSphere))
  (:Pressed
    (CallFunction|SetStunt true)
    (Physics|AddImpulse _helisphere "0, 0,1000.000000" "None" true)
    (Class|PrimitiveComponent|AddAngularImpulseinDegrees _helisphere (* (.Forward (Utilities|ControllerForwardRightV)) (Math|Random|RandomFloatinRange 2.5e+02 7.5e+02)) "None" true)
    (Utilities|FlowControl|Delay 1.0)
    (CallFunction|SetStunt false)))

(fn ConstructionScript)

(fn HoverUpdate
  (bind _helisphere (Variables|Components|GetHeliSphere))
  (bind _helisphere_2 (Variables|Components|GetHeliSphere))
  (bind _returnvalue (Transformation|GetWorldLocation _helisphere))
  (bind (_outhit _returnvalue_2) (Collision|LineTraceByChannel _returnvalue (+ _returnvalue (* (Math|Vector|NegateVector (Math|Vector|GetUpVector "0, 0, 0")) (Variables|Physics|GetTraceLength))) "TraceTypeQuery2" true 0 "None"))
  (if _returnvalue_2
    (Physics|NewHitActor (.HitActor (Collision|BreakHitResult _outhit)) (+ (.Distance (Collision|BreakHitResult _outhit)) 5e+01))
    (Variables|Physics|SetMinTraceLength (+ (.Distance (Collision|BreakHitResult _outhit)) 5e+01))
    (Variables|Physics|SetMaxTraceLength (+ (.Distance (Collision|BreakHitResult _outhit)) 4e+03))
    (Physics|AddForce _helisphere_2 (* (.ImpactNormal (Collision|BreakHitResult _outhit)) (Math|Float|Lerp (Variables|Physics|GetHoverForce) 0.0 (/ (Math|Vector|VectorLength (- (.Location (Collision|BreakHitResult _outhit)) _returnvalue)) (Variables|Physics|GetTraceLength)))) "None" false)
    (Class|PrimitiveComponent|SetLinearDamping _helisphere_2 (Variables|Physics|GetLinearDamping))
    (Class|PrimitiveComponent|SetAngularDamping _helisphere_2 (Variables|Physics|GetAngularDamping))))

(fn Move
  (params (Sphere :type Primitive%20Component%20Object%20Reference) (Vector :type Vector))
  (Physics|AddForce Sphere Vector "None" true))

(fn Stabilize
  (params (Alpha :type Float%20%28single-precision%29))
  (bind _lerprotation (Variables|Physics|GetLerpRotation))
  (bind _helisphere (Variables|Components|GetHeliSphere))
  (bind _returnvalue (Transformation|GetWorldRotation _helisphere))
  (if (not (Variables|Physics|GetStunt))
    (Transformation|SetWorldRotation _helisphere (Math|Rotator|Lerp(Rotator) (Math|Rotator|MakeRotator (.roll _returnvalue) (.pitch _returnvalue) (.yaw _returnvalue)) (Math|Rotator|MakeRotator (.roll _lerprotation) (.pitch _lerprotation) (.yaw _lerprotation)) (* Alpha (Variables|Physics|GetLerpSpeed))) false false)))

(fn InputMove
  (bind (_forward _right) (Utilities|ControllerForwardRightV))
  (bind _returnvalue (Math|Vector|NegateVector _right))
  (bind _returnvalue_2 (Math|Vector|NegateVector _forward))
  (if (Math|Boolean|ORBoolean (Variables|Input|GetbW) (Variables|Input|GetbA) (Variables|Input|GetbS) (Variables|Input|GetbD))
    (Variables|Physics|SetLerpRotation "0, 0, 0")
    (Utilities|FlowControl|Sequence
      (:then_0
        (Input|MoveForward _forward _right))
      (:then_1
        (Input|MoveBack _returnvalue_2 _returnvalue))
      (:then_2
        (Input|MoveRight _right _returnvalue_2))
      (:then_3
        (Input|MoveLeft _returnvalue _forward)))
    (else
      (Physics|LerpRotationDrone "0, 0, 0"))))

(fn NewHitActor
  (params (NewHitActor :type Actor%20Object%20Reference) (Distance :type Float%20%28single-precision%29))
  (if (not (Variables|Physics|GetStunt))
    (bind _output_get (LocalVariables|SetOldHitActor (Variables|Physics|GetHitActor)))
    (if (!= NewHitActor _output_get)
      (Variables|Physics|SetHitActor NewHitActor)
      (Variables|Physics|SetTraceLength Distance))))

(fn AppendDistance
  (bind _distance (Utilities|GetLengthtoLastDistance))
  (Variables|/Script/Engine.RotatingMovementComponent|SetRotationRate (Variables|Default|GetMultiRotatingMovement) (Math|Rotator|MakeRotator 0.0 0.0 (Math|Float|Clamp(Float) (* _distance 1.5e+02) 1.7e+02 1.2e+03)))
  (Variables|Stats|SetDistance (+ (Variables|Stats|GetDistance) _distance))
  (Variables|Physics|SetLastLocation (Transformation|GetWorldLocation (Variables|Components|GetHeliSphere))))

(fn InputUpDown
  (Utilities|FlowControl|Sequence
    (:then_0
      (if (Variables|Input|GetbSpace)
        (if (<= (+ (Variables|Physics|GetTraceLength) 25.0) (Variables|Physics|GetMaxTraceLength))
          (Variables|Physics|SetTraceLength (+ (Variables|Physics|GetTraceLength) 25.0)))))
    (:then_1
      (if (Variables|Input|GetbCtrl)
        (if (>= (- (Variables|Physics|GetTraceLength) 25.0) (Variables|Physics|GetMinTraceLength))
          (Variables|Physics|SetTraceLength (- (Variables|Physics|GetTraceLength) 25.0)))))))

(fn LerpRotationDrone
  (params (Axis :type Vector))
  (if (Math|Vector|Equal(Vector) Axis "0, 0, 0" 1.0)
    (Variables|Physics|SetLerpRotation "0, 0, 0"))
  (Variables|Physics|SetLerpRotation (Math|Rotator|CombineRotators (Variables|Physics|GetLerpRotation) (Math|Vector|RotatorfromAxisandAngle Axis 25.0))))

(fn MoveLeft
  (params (LeftV :type Vector) (ForwardV :type Vector))
  (if (Variables|Input|GetbA)
    (Physics|LerpRotationDrone ForwardV)
    (Input|Move (Variables|Components|GetHeliSphere) (* LeftV 1e+03))))

(fn MoveRight
  (params (RightV :type Vector) (BackV :type Vector))
  (if (Variables|Input|GetbD)
    (Physics|LerpRotationDrone BackV)
    (Input|Move (Variables|Components|GetHeliSphere) (* RightV 1e+03))))

(fn MoveBack
  (params (BackV :type Vector) (LeftV :type Vector))
  (if (Variables|Input|GetbS)
    (Physics|LerpRotationDrone LeftV)
    (Input|Move (Variables|Components|GetHeliSphere) (* BackV 1e+03))))

(fn MoveForward
  (params (ForwardV :type Vector) (RightV :type Vector))
  (if (Variables|Input|GetbW)
    (Physics|LerpRotationDrone RightV)
    (Input|Move (Variables|Components|GetHeliSphere) (* ForwardV 1e+03))))

(fn ScanSurroundings
  (bind _helisphere (Variables|Components|GetHeliSphere))
  (bind _returnvalue (Transformation|GetWorldLocation _helisphere))
  (bind _output_get (LocalVariables|SetScanCount (Math|Random|RandomIntegerinRange 0 25)))
  (for _index (range 0 _output_get)
    (if (Math|Random|RandomBoolwithWeight 0.2)
      (bind (_outhit _returnvalue_2) (Collision|LineTraceByChannel _returnvalue (+ _returnvalue (* (Math|Vector|RotateVectorAroundAxis (Math|Vector|GetForwardVector "0, 0, 0") (Math|Random|RandomFloatinRange 0.0 3.6e+02) (Math|Vector|GetUpVector "0, 0, 0")) 5e+03)) "TraceTypeQuery1" false 0 "None"))
      (if _returnvalue_2
        (Math|Integer|IncrementInt (Variables|Stats|GetProbesCount)
          (:%20%20
            (bind _returnvalue_3 (Effects|SpawnEmitteratLocation "/Game/Blueprints/Gameplay/VFX/PS_Beam_Scan.PS_Beam_Scan" (.TraceStart (Collision|BreakHitResult _outhit))))
            (Class|ParticleSystemComponent|SetBeamSourcePoint _returnvalue_3 0 (.TraceStart (Collision|BreakHitResult _outhit)))
            (Class|ParticleSystemComponent|SetBeamEndPoint _returnvalue_3 0 (.ImpactPoint (Collision|BreakHitResult _outhit)))
            (if (< (.Distance (Collision|BreakHitResult _outhit)) 75.0)
              (Effects|Components|ParticleSystem|SetColorParameter _returnvalue_3 "Color" "(R=0.625000,G=0.460351,B=0.441665,A=1.000000)")
              (Physics|AddForce (Variables|Components|GetHeliSphere) (* (Math|Vector|NegateVector (Math|Vector|GetUnitDirection(Vector) (.TraceStart (Collision|BreakHitResult _outhit)) (.ImpactPoint (Collision|BreakHitResult _outhit)))) 1e+04) "None" true)
              (else
                (Effects|Components|ParticleSystem|SetColorParameter _returnvalue_3 "Color" "(R=0.503924,G=0.625000,B=0.484761,A=1.000000)")))))))))

(fn SetActive
  (params (NewActive :type Boolean))
  (bind _output_get (Variables|Physics|SetActive NewActive))
  (for _array_element (Variables|Trail|GetTrails)
    (Effects|Components|ParticleSystem|SetEmitterEnable _array_element "Trail" _output_get)))

(fn UpdateColor
  (if (Variables|Physics|GetActive)
    (Variables|Color|SetTint (Utilities|Struct|MakeSlateColor "(R=0.000000,G=1.000000,B=0.380774,A=1.000000)"))
    (if (Variables|Physics|GetStunt)
      (Variables|Color|SetTint (Utilities|Struct|MakeSlateColor "(R=1.000000,G=0.000000,B=0.655376,A=1.000000)")))
    (else
      (Variables|Color|SetTint (Utilities|Struct|MakeSlateColor "(R=1.000000,G=0.034090,B=0.000000,A=1.000000)")))))

(fn ColorImplementation
  (bind _tint (Variables|Color|GetTint))
  (bind _specifiedcolor (Utilities|Struct|BreakSlateColor _tint))
  (bind (_r _g _b) (Math|Color|BreakColor _specifiedcolor))
  (for _array_element (Utilities|Array|MakeArray (Variables|Default|GetPointLight) (Variables|Default|GetPointLight1) (Variables|Default|GetPointLight2) (Variables|Default|GetPointLight3))
    (Rendering|Components|Light|SetLightColor _array_element (Utilities|Struct|BreakSlateColor (Variables|Color|GetTint)) true))
  (for _array_element_2 (Variables|Trail|GetTrails)
    (Rendering|Material|GetVectorParameterValue (.Value (Utilities|Map|Find (Variables|Trail|GetTrailMaterials) _array_element_2)) "EmissiveColor" :!class /Script/Engine.MaterialInstanceDynamic)
    (Rendering|Material|SetVectorParameterValue (.Value (Utilities|Map|Find (Variables|Trail|GetTrailMaterials) _array_element_2)) "EmissiveColor" (Utilities|Struct|MakeLinearColor (* _r 1e+02) (* _g 1e+02) (* _b 1e+02) 1.0) :!class /Script/Engine.MaterialInstanceDynamic)))

(fn SetStunt
  (params (Stunt :type Boolean))
  (bind _output_get (Variables|Physics|SetStunt Stunt))
  (Variables|Default|SetSoundInterpTo (select _output_get 0.7 0.1)))

(fn SoundInterp
  (params (DeltaTime :type Float%20%28single-precision%29))
  (bind _loop (Variables|Default|GetLoop))
  (Audio|Components|Audio|SetPitchMultiplier _loop (Math|Float|Lerp (Variables|/Script/Engine.AudioComponent|GetPitchMultiplier _loop) (Variables|Default|GetSoundInterpTo) (* DeltaTime 3.0))))

(fn AddDataProgress
  (if (< (Variables|Default|GetCollectedDataProgress) 1e+02)
    (bind _output_get (Variables|Default|SetCollectedDataProgress (+ (Variables|Default|GetCollectedDataProgress) 0.1)))
    (Transformation|SetWorldScale3D (Variables|Default|GetDataAbsorber) (Math|Vector|Lerp(Vector) "0, 0, 0" "0.800000,0.800000,0.800000" (* _output_get 0.01)))
    (Rendering|Material|SetScalarParameterValue (Variables|Default|GetDataAbsorbMaterial) "Alpha" (* _output_get 0.01) :!class /Script/Engine.MaterialInstanceDynamic)
    (if (>= _output_get 1e+02)
      (Variables|Default|SetCollectedDataProgress 1e+02)
      (Variables|Default|SetbCollectedData true))))

(fn AddEncryptionProgress
  (if (< (Variables|Default|GetEncryptedDataProgress) 1e+02)
    (bind _output_get (Variables|Default|SetEncryptedDataProgress (+ (Variables|Default|GetEncryptedDataProgress) 0.1)))
    (Transformation|SetWorldScale3D (Variables|Default|GetDataAbsorber) (Math|Vector|Lerp(Vector) "0.800000,0.800000,0.800000" "0, 0, 0" (* _output_get 0.01)))
    (Rendering|Material|SetScalarParameterValue (Variables|Default|GetDataAbsorbMaterial) "Alpha" (Class|UtilityLibrary|SetScalePure (* _output_get 0.01) 0.0 1.0 1.0 0.0) :!class /Script/Engine.MaterialInstanceDynamic)
    (if (>= _output_get 1e+02)
      (Variables|Default|SetEncryptedDataProgress 1e+02)
      (Variables|Default|SetbEncryptedData true))))

(fn KeepWingsZeroRotation
  (for _array_element (Utilities|Array|MakeArray (Variables|Default|GetBladePivot_2) (Variables|Default|GetBladePivot) (Variables|Default|GetBladePivot_4) (Variables|Default|GetBladePivot_3))
    (Transformation|SetWorldRotation _array_element (Math|Rotator|Lerp(Rotator) (Transformation|GetWorldRotation _array_element) "0, 0, 0" 0.1 true) false false)))