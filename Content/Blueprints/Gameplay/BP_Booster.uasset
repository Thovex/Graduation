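; BP_Booster is a two-way booster that launches BP_HeliSphere actors along its forward or backward arrow.
; Forward and Backward triggers apply a randomized mass-independent force, disabling the opposite trigger until a two-second reset.
; ForwardLerp and BackLerp volumes run looping frame-delta timers, apparently easing the sphere toward their centers via location lerps.
; Each lerp volume disables its counterpart until overlap ends.
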(event OnComponentBeginOverlap(ForwardLerp)
  (params (OverlappedComponent :type Primitive%20Component%20Object%20Reference) (OtherActor :type Actor%20Object%20Reference) (OtherComp :type Primitive%20Component%20Object%20Reference) (OtherBodyIndex :type Integer) (bFromSweep :type Boolean) (SweepResult :type Hit%20Result%20Structure%20%28by%20ref%29))
  (bind _asbp_heli_sphere (Utilities|IsHelisphere OtherActor))
  (Variables|Default|SetHeliSphere _asbp_heli_sphere)
  (Collision|SetCollisionEnabled (Variables|Default|GetBackLerp) "NoCollision")
  (bind _returnvalue (Utilities|Time|SetTimerbyEvent (EventDispatchers|CreateEvent :!event Custom|LerpToForward) (Utilities|Time|GetWorldDeltaSeconds) true))
  (Variables|Default|SetTimerHandle _returnvalue))

(event OnComponentBeginOverlap(BackLerp)
  (params (OverlappedComponent :type Primitive%20Component%20Object%20Reference) (OtherActor :type Actor%20Object%20Reference) (OtherComp :type Primitive%20Component%20Object%20Reference) (OtherBodyIndex :type Integer) (bFromSweep :type Boolean) (SweepResult :type Hit%20Result%20Structure%20%28by%20ref%29))
  (bind _asbp_heli_sphere (Utilities|IsHelisphere OtherActor))
  (Variables|Default|SetHeliSphere _asbp_heli_sphere)
  (Collision|SetCollisionEnabled (Variables|Default|GetForwardLerp) "NoCollision")
  (bind _returnvalue (Utilities|Time|SetTimerbyEvent (EventDispatchers|CreateEvent :!event Custom|LerpToBackward) (Utilities|Time|GetWorldDeltaSeconds) true))
  (Variables|Default|SetTimerHandle _returnvalue))

(event OnComponentEndOverlap(BackLerp)
  (params (OverlappedComponent :type Primitive%20Component%20Object%20Reference) (OtherActor :type Actor%20Object%20Reference) (OtherComp :type Primitive%20Component%20Object%20Reference) (OtherBodyIndex :type Integer))
  (Utilities|IsHelisphere OtherActor)
  (Utilities|Time|ClearandInvalidateTimerbyHandle (Variables|Default|GetTimerHandle))
  (Collision|SetCollisionEnabled (Variables|Default|GetForwardLerp) "QueryAndPhysics"))

(event OnComponentBeginOverlap(Forward)
  (params (OverlappedComponent :type Primitive%20Component%20Object%20Reference) (OtherActor :type Actor%20Object%20Reference) (OtherComp :type Primitive%20Component%20Object%20Reference) (OtherBodyIndex :type Integer) (bFromSweep :type Boolean) (SweepResult :type Hit%20Result%20Structure%20%28by%20ref%29))
  (bind _asbp_heli_sphere (Utilities|IsHelisphere OtherActor))
  (Variables|Default|SetHeliSphere _asbp_heli_sphere)
  (Collision|SetCollisionEnabled (Variables|Default|GetBackward) "NoCollision")
  (CallFunction|ApplyForce true)
  (Utilities|FlowControl|Delay 2.0)
  (CallFunction|Reset))

(event OnComponentEndOverlap(ForwardLerp)
  (params (OverlappedComponent :type Primitive%20Component%20Object%20Reference) (OtherActor :type Actor%20Object%20Reference) (OtherComp :type Primitive%20Component%20Object%20Reference) (OtherBodyIndex :type Integer))
  (Utilities|IsHelisphere OtherActor)
  (Utilities|Time|ClearandInvalidateTimerbyHandle (Variables|Default|GetTimerHandle))
  (Collision|SetCollisionEnabled (Variables|Default|GetBackLerp) "QueryAndPhysics"))

(event OnComponentBeginOverlap(Backward)
  (params (OverlappedComponent :type Primitive%20Component%20Object%20Reference) (OtherActor :type Actor%20Object%20Reference) (OtherComp :type Primitive%20Component%20Object%20Reference) (OtherBodyIndex :type Integer) (bFromSweep :type Boolean) (SweepResult :type Hit%20Result%20Structure%20%28by%20ref%29))
  (bind _asbp_heli_sphere (Utilities|IsHelisphere OtherActor))
  (Variables|Default|SetHeliSphere _asbp_heli_sphere)
  (Collision|SetCollisionEnabled (Variables|Default|GetForward) "NoCollision")
  (CallFunction|ApplyForce false)
  (Utilities|FlowControl|Delay 2.0)
  (CallFunction|Reset))

(event Custom|Reset
  (Collision|SetCollisionEnabled (Variables|Default|GetBackward) "QueryAndPhysics")
  (Collision|SetCollisionEnabled (Variables|Default|GetForward) "QueryAndPhysics"))

(event Custom|ApplyForce
  (params (Forward :type Boolean))
  (Physics|AddForce (Variables|/Game/Blueprints/Gameplay/BP_HeliSphere.BP_HeliSphere_C|GetHeliSphere (Variables|Default|GetHeliSphere)) (* (Math|Vector|GetForwardVector (select Forward (Variables|Default|GetForwardArrow) (Variables|Default|GetBackwardArrow))) (Math|Random|RandomFloatinRange 8e+03 1.5e+04)) "None" true))

(event Custom|LerpToForward
  (Transformation|SetActorLocation (Variables|Default|GetHeliSphere) (Math|Vector|Lerp(Vector) (Transformation|GetActorLocation (Variables|Default|GetHeliSphere)) (Transformation|GetWorldLocation (Variables|Default|GetForwardLerp)) 0.05) false false))

(event Custom|LerpToBackward
  (Transformation|SetActorLocation (Variables|Default|GetHeliSphere) (Math|Vector|Lerp(Vector) (Transformation|GetActorLocation (Variables|Default|GetHeliSphere)) (Transformation|GetWorldLocation (Variables|Default|GetBackLerp)) 0.05) false false))

(fn ConstructionScript)